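; Networked PaperZD player character with jumping, falling, attacks, bow charging and a nickname widget.
; Server events set state flags, whose OnRep handlers trigger jumps and send animation-instance messages, with NextAttack selecting the combo.
; A hitbox, hidden and disabled at BeginPlay, damages other player characters on overlap.
; Nicknames pass through a server-to-multicast event, with a delayed one-time send from Tick while waiting for the name.
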(event OnComponentBeginOverlap(CollisionBox)
  (params (OverlappedComponent :type Primitive%20Component%20Object%20Reference) (OtherActor :type Actor%20Object%20Reference) (OtherComp :type Primitive%20Component%20Object%20Reference) (OtherBodyIndex :type Integer) (bFromSweep :type Boolean) (SweepResult :type Hit%20Result%20Structure%20%28by%20ref%29))
  ;[1 1 1] Apply damage on box hit
  (bind _asbp_main_paper_zdcharacter (Utilities|Casting|CastToBP_MainPaperZDCharacter OtherActor))
  (Utilities|IsValid _asbp_main_paper_zdcharacter
    (:Is%20Valid
      (Game|Damage|ApplyDamage _asbp_main_paper_zdcharacter 1e+01 (Game|GetPlayerController 0) self "/Script/Engine.DamageType"))))

(event Custom|SERVER_Jump
  ;[1 1 1] Jumping
  (Variables|Default|SetIsJumping true))

(event Custom|SERVER_StopJumping
  ;[1 1 1] Jumping
  (Variables|Default|SetIsJumping false))

(event Custom|SERVER_Attack
  ;[1 1 1] Attack
  (Variables|Default|SetNextAttack "NewEnumerator1")
  (Variables|Default|SetIsAttacking true))

(event Custom|SERVER_StopAttack
  ;[1 1 1] Attack
  (Variables|Default|SetIsAttacking false))

(event Custom|SERVER_SetNickName
  (params (PlayerName :type Text))
  (CallFunction|MULTICASTSetNickName PlayerName))

(event Custom|MULTICAST_SetNickName
  (params (PlayerName :type Text))
  (Variables|Default|SetNickName PlayerName))

(event Custom|SERVER_Fall
  ;[1 1 1] Jumping
  (Variables|Default|SetIsFalling true))

(event Custom|SERVER_ChargeBow
  ;[1 1 1] Attack
  (Variables|Default|SetNextAttack "NewEnumerator2")
  (Variables|Default|SetIsAttacking true))

(event Custom|SERVER_ShootBow
  ;[1 1 1] Attack
  (Variables|Default|SetIsAttacking false))

(event EventBeginPlay
  (CallFunction|HideHitBox))

(event EventTick
  (params (DeltaSeconds :type Float%20%28single-precision%29))
  (if (Variables|Default|GetWaitingForNickName)
    (Utilities|FlowControl|DoOnce false
      (:Completed
        (Utilities|FlowControl|Delay 0.1)
        (CallFunction|SERVERSetNickName (Variables|Default|GetNickName))))))

(event EventOnLanded
  (params (Hit :type Hit%20Result%20Structure%20%28by%20ref%29))
  ;[1 1 1] Jumping
  (Variables|Default|SetIsFalling false))

(event EventJumpPlayer
  ;[1 1 1] Jumping
  (CallFunction|SERVERJump))

(event EventOnWalkingOffLedge
  (params (PreviousFloorImpactNormal :type Vector%20%28by%20ref%29 :default "0, 0, 0") (PreviousFloorContactNormal :type Vector%20%28by%20ref%29 :default "0, 0, 0") (PreviousLocation :type Vector%20%28by%20ref%29 :default "0, 0, 0") (TimeDelta :type Float%20%28single-precision%29))
  ;[1 1 1] Jumping
  (CallFunction|SERVERFall))

(event EventAttack
  ;[1 1 1] Attack
  (CallFunction|SERVERAttack))

(event EventStopAttack
  ;[1 1 1] Attack
  (CallFunction|SERVERStopAttack))

(event EventStopPlayerJumping
  ;[1 1 1] Jumping
  (CallFunction|SERVERStopJumping))

(event EventChargeBow
  ;[1 1 1] Attack
  (CallFunction|SERVERChargeBow))

(event EventShootBow
  ;[1 1 1] Attack
  (CallFunction|SERVERShootBow))

(fn ConstructionScript)

(fn OnRepIsJumping
  (if (and (Variables|Default|GetIsJumping) (Character|CanJump))
    (Character|Jump)
    (Class|BPIStateRequest|JumpStateRequest(Message) (Variables|/Script/PaperZD.PaperZDAnimationComponent|GetAnimInstance (Variables|Default|GetAnimationComponent)) "JumpActivated" "Locomotion")))

(fn OnRepIsAttacking
  (if (Variables|Default|GetIsAttacking)
    (Class|BPIComboRequest|RequestCombo(Message) (Variables|/Script/PaperZD.PaperZDAnimationComponent|GetAnimInstance (Variables|Default|GetAnimationComponent)) (Variables|Default|GetNextAttack))))

(fn SetUsername
  (params (PlayerName :type Text)))

(fn HideHitBox
  (bind _collisionbox (Variables|Default|GetCollisionBox))
  (Collision|SetCollisionEnabled _collisionbox "NoCollision")
  (Development|SetHiddeninGame _collisionbox true false))

(fn SetNIckName
  (params (PlayerName :type Text))
  (bind _usernamewidget (Variables|Default|GetUsernameWidget))
  (if (Class|WidgetComponent|IsWidgetVisible _usernamewidget)
    (bind _aswbp_username (Utilities|Casting|CastToWBP_Username (UserInterface|GetWidget _usernamewidget)))
    (Class|UsernameUserWidget|SetPlayerName _aswbp_username PlayerName)
    (Variables|Default|SetWaitingForNickName false)
    (else
      (Variables|Default|SetWaitingForNickName true)
      (Variables|Default|SetNickName PlayerName))))

(fn OnRepIsFalling
  (if (Variables|Default|GetIsFalling)
    (Class|BPIStateRequest|FallStateRequest(Message) (Variables|/Script/PaperZD.PaperZDAnimationComponent|GetAnimInstance (Variables|Default|GetAnimationComponent)) "Falling" "Locomotion")))

(fn OnRepIsChargingBow
  (if (Variables|Default|GetIsChargingBow)
    (Class|BPIComboRequest|RequestCombo(Message) (Variables|/Script/PaperZD.PaperZDAnimationComponent|GetAnimInstance (Variables|Default|GetAnimationComponent)) "NewEnumerator2")))