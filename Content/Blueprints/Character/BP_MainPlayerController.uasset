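; Player controller that syncs the player's name, opens the in-game menu and provides a dash for the Paper2D character.
; After a short replication delay on BeginPlay, it passes the game instance's saved name through a server request to the player state.
; ShowMenu lazily creates the menu widget and switches to UI-only input.
; PlayerDash launches the character along its forward vector, scaled by sprite X scale, with a brief cooldown.
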(event Custom|SERVER_RequestNameChange
  (params (NewPlayerName :type Text))
  (bind _asbp_main_player_player_state (Utilities|Casting|CastToBP_MainPlayerPlayerState (Variables|Default|GetPlayerState self)))
  (Default|SERVERUpdateName _asbp_main_player_player_state NewPlayerName))

(event EventBeginPlay
  (Utilities|FlowControl|Delay 0.2) ; Wait for replication variables to be replicated and initialized
  (bind _asbp_main_game_instance (Utilities|Casting|CastToBP_MainGameInstance (Game|GetGameInstance)))
  (CallFunction|SERVERRequestNameChange (Variables|/Script/Combat2DGame.MainGameInstance|GetPlayerName _asbp_main_game_instance)))

(event EventShowMenu
  (if (Utilities|IsValid (Variables|Default|GetInGameMenu))
    _
    (else
      (bind _returnvalue (UserInterface|CreateWidget "/Game/UI/WBP_InGameMenu.WBP_InGameMenu_C" (Game|GetPlayerController 0)))
      (bind _output_get (Variables|Default|SetInGameMenu _returnvalue))))
  (UserInterface|Viewport|AddtoViewport _output_get 0)
  (Input|SetInputModeUIOnly self _output_get "LockInFullscreen" false)
  (Variables|Default|SetbShowMouseCursor true))

(fn ConstructionScript)